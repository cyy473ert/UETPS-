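; A door actor that the player opens and closes with E, provided the key-pickup flag (是否捡到钥匙) is true.
; Overlapping its Box trigger enables input, shows the mouse cursor and opens a Gate; leaving reverses all three.
; E passes through the Gate to a FlipFlop that alternately plays and reverses a Timeline driving the door's relative yaw.
; Without the key, E prints a "no key" message.
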(event OnComponentBeginOverlap(Box)
  (params (OverlappedComponent :type Primitive%20Component%20Object%20Reference) (OtherActor :type Actor%20Object%20Reference) (OtherComp :type Primitive%20Component%20Object%20Reference) (OtherBodyIndex :type Integer) (bFromSweep :type Boolean) (SweepResult :type Hit%20Result%20Structure%20%28by%20ref%29))
  (bind _returnvalue (Game|GetPlayerController 0))
  (Variables|/Script/Engine.PlayerController|SetbShowMouseCursor _returnvalue true)
  (Input|EnableInput _returnvalue)
  (Utilities|FlowControl|Gate true) ; enters at Open
)

(event OnComponentEndOverlap(Box)
  (params (OverlappedComponent :type Primitive%20Component%20Object%20Reference) (OtherActor :type Actor%20Object%20Reference) (OtherComp :type Primitive%20Component%20Object%20Reference) (OtherBodyIndex :type Integer))
  (bind _returnvalue (Game|GetPlayerController 0))
  (Variables|/Script/Engine.PlayerController|SetbShowMouseCursor _returnvalue false)
  (Input|DisableInput _returnvalue)
  (Utilities|FlowControl|Gate true) ; enters at Close
)

(event EventBeginPlay)

(event Collision|EventActorBeginOverlap
  (params (OtherActor :type Actor%20Object%20Reference)))

(event EventTick
  (params (DeltaSeconds :type Float%20%28single-precision%29)))

(event Input|KeyboardEvents|E
  (params (Key :type Key%20Structure :default "None"))
  (:Pressed
    (if (Variables|Default|Get是否捡到钥匙)
      (Utilities|FlowControl|Gate true
        (:Exit
          (Utilities|FlowControl|FlipFlop
            (:A
              (bind _开关门 (Timeline|时间轴 Play)
                (:Update
                  (Transformation|SetRelativeRotation (Variables|Default|Get门) (Math|Rotator|MakeRotator 0.0 0.0 _开关门) false false))))
            (:B
              (Timeline|时间轴 Reverse)))))
      (else
        (Development|PrintString "没有钥匙")))))

(fn ConstructionScript)